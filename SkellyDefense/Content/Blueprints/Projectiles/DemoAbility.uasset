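; DemoAbility is an explosive ability actor, filed under projectiles, that deals area damage to enemies.
; On explosion it spawns a large particle effect on both authority and remote, then hides itself and disables collision.
; Only the authority runs a sphere overlap for pawns and applies damage to those tagged Enemy, crediting the instigator's controller.
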(event `self.OnExplosion`
  (`/Engine/EditorBlueprintResources/ActorMacros.Switch Has Authority`
    (:`Authority`
      (bind _outactors (`KismetSystemLibrary.SphereOverlapActors_NEW` (`self.K2_GetActorLocation`) 500.0 (`|MakeArray` "ObjectTypeQuery3" :!type "EObjectTypeQuery Enum")))
      (`GameplayStatics.SpawnEmitterAtLocation` "/Game/StarterContent/Particles/BiggerExplosion.BiggerExplosion" (`self.K2_GetActorLocation`))
      (for _array_element _outactors
        (if (`self.ActorHasTag` _array_element "Enemy")
          (`GameplayStatics.ApplyDamage` _array_element 100.0 (`self.GetInstigatorController`) self "/Script/Engine.DamageType"))))
    (:`Remote`
      (`GameplayStatics.SpawnEmitterAtLocation` "/Game/StarterContent/Particles/BiggerExplosion.BiggerExplosion" (`self.K2_GetActorLocation`))))
  (`self.SetActorHiddenInGame` true)
  (`self.SetActorEnableCollision` false))

(fn `UserConstructionScript`)