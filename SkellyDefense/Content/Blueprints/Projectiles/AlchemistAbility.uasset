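; AlchemistAbility is a projectile actor that applies a slow to boulders and enemies it overlaps, handled only on the server.
; A Boulder hit slows that boulder alone, while an Enemy hit sphere-queries nearby BasicEnemy pawns for an area slow.
; Each slow sets the target's Slowed flag and resets its SlowedTimer.
; After either hit, the projectile is hidden and loses collision instead of being destroyed.
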(event `self.OnExplosion`)

(event `self.ReceiveActorBeginOverlap`
  (params (OtherActor :type "Actor Object Reference"))
  (`/Engine/EditorBlueprintResources/ActorMacros.Switch Has Authority`
    (:`Authority`
      (bind _output_get (set `self.HitActor` OtherActor))
      (if (`self.ActorHasTag` _output_get "Boulder")
        (bind _asboulder_bp (cast `/Game/Blueprints/Enemies/Boulder_BP` (`self.HitActor`)))
        (set `/Game/Blueprints/Enemies/Boulder_BP.Slowed` true _asboulder_bp)
        (set `/Game/Blueprints/Enemies/Boulder_BP.SlowedTimer` 0.0 _asboulder_bp)
        (`self.SetActorHiddenInGame` true :!label _label)
        (`self.SetActorEnableCollision` false)
        (elif (`self.ActorHasTag` _output_get "Enemy")
          (bind _outactors (`KismetSystemLibrary.SphereOverlapActors_NEW` (`self.K2_GetActorLocation`) 250.0 (`|MakeArray` "ObjectTypeQuery3" :!type "EObjectTypeQuery Enum") "/Script/SkellyDefense.BasicEnemy"))
          (for _array_element _outactors
            (bind _asbasic_enemy (cast `BasicEnemy` _array_element))
            (set `BasicEnemy.Slowed` true _asbasic_enemy)
            (set `BasicEnemy.SlowedTimer` 0.0 _asbasic_enemy))
          (goto _label))))))

(event `self.ReceiveTick`
  (params (DeltaSeconds :type "Float (single-precision)")))

(fn `UserConstructionScript`)