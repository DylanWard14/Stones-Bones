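; Fireball projectile that explodes to damage nearby enemies.
; On explosion, the authority runs a sphere overlap for pawns and applies damage to those tagged "Enemy", while both authority and remote spawn the explosion particle effect.
; The fireball then hides and disables collision rather than being destroyed.
; An unconnected older version using radial damage with walls and machine gunners ignored remains in the graph.
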(event `self.OnExplosion`
  (`/Engine/EditorBlueprintResources/ActorMacros.Switch Has Authority`
    (:`Authority`
      (bind _outactors (`KismetSystemLibrary.SphereOverlapActors_NEW` (`self.K2_GetActorLocation`) 100.0 (`|MakeArray` "ObjectTypeQuery3" :!type "EObjectTypeQuery Enum")))
      (`GameplayStatics.SpawnEmitterAtLocation` "/Game/StarterContent/Particles/P_Explosion.P_Explosion" (`self.K2_GetActorLocation`))
      (for _array_element _outactors
        (if (`self.ActorHasTag` _array_element "Enemy")
          (`GameplayStatics.ApplyDamage` _array_element 50.0 (`self.GetInstigatorController`) self "/Script/Engine.DamageType"))))
    (:`Remote`
      (`GameplayStatics.SpawnEmitterAtLocation` "/Game/StarterContent/Particles/P_Explosion.P_Explosion" (`self.K2_GetActorLocation`))))
  (`self.SetActorHiddenInGame` true)
  (`self.SetActorEnableCollision` false))

(event `self.ReceiveTick`
  (params (DeltaSeconds :type "Float (single-precision)")))

(fn `UserConstructionScript`)