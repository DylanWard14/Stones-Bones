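; Boulder projectile Blueprint that supports a temporary slowed state on its ProjectileMovement component.
; On Tick with authority, an externally set Slowed flag caps the speed low and removes gravity while a timer accumulates.
; After three seconds it clears the flag, restores speed cap and gravity, and relaunches along local forward.
; The timer is never reset here, and normal movement values are reapplied every unslowed tick.
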(event `self.ReceiveTick`
  (params (DeltaSeconds :type "Float (single-precision)"))
  (bind _projectilemovement (`self.ProjectileMovement`))
  (bind _projectilemovement_2 (`self.ProjectileMovement`))
  (bind _projectilemovement_3 (`self.ProjectileMovement`))
  (`/Engine/EditorBlueprintResources/ActorMacros.Switch Has Authority`
    (:`Authority`
      (if (`self.Slowed`)
        (set `self.SlowedTimer` (+ DeltaSeconds (`self.SlowedTimer`)))
        (set `ProjectileMovementComponent.MaxSpeed` 100.0 _projectilemovement)
        (set `ProjectileMovementComponent.ProjectileGravityScale` 0.0 _projectilemovement)
        (if (>= (`self.SlowedTimer`) 3.0)
          (set `self.Slowed` false)
          (set `ProjectileMovementComponent.MaxSpeed` 1500.0 _projectilemovement_2)
          (set `ProjectileMovementComponent.ProjectileGravityScale` 0.5 _projectilemovement_2)
          (`ProjectileMovementComponent.SetVelocityInLocalSpace` _projectilemovement_2 (1000.0 0.0 0.0)))
        (else
          (set `ProjectileMovementComponent.MaxSpeed` 1500.0 _projectilemovement_3)
          (set `ProjectileMovementComponent.ProjectileGravityScale` 0.5 _projectilemovement_3))))))

(fn `UserConstructionScript`)