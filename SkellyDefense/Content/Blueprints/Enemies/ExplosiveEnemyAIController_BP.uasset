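; AI controller for a suicide-bomber enemy that chases a random SkellyDefenseCharacter chosen at BeginPlay.
; MoveTowardsTarget re-triggers itself each second, issuing a server-side AI move to within the pawn's attack radius.
; On arrival it deals full radial damage using the pawn's AttackDamage, then PlayExplosion sets the ExplosiveEnemy_BP's Health negative.
; The emitter-and-destroy explosion logic is disconnected, and the stored MainBuilding is never targeted.
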(event `self.ReceiveBeginPlay`
  (bind _outactors (`GameplayStatics.GetAllActorsOfClass` "/Script/SkellyDefense.MainBuilding"))
  (set `self.MainBuilding` (`KismetArrayLibrary.Array_Get` _outactors))
  (bind _outactors_2 (`GameplayStatics.GetAllActorsOfClass` "/Script/SkellyDefense.SkellyDefenseCharacter"))
  (bind _output_get (set `self.Players` _outactors_2))
  (set `self.Target` (`KismetArrayLibrary.Array_Get` _output_get (`KismetMathLibrary.RandomIntegerInRange` 0 (- (`KismetArrayLibrary.Array_Length` (`self.Players`)) 1))))
  (`KismetSystemLibrary.Delay` 1.0)
  (set `self.DamageAmount` (`BasicEnemy.AttackDamage` (cast `BasicEnemy` (`self.K2_GetPawn`) :!pure true))))

(event `self.ReceiveTick`
  (params (DeltaSeconds :type "Float (single-precision)")))

(event `MoveTowardsTarget`
  (`KismetSystemLibrary.K2_SetTimerDelegate` (delegate `MoveTowardsTarget`) 1.0)
  (`/Engine/EditorBlueprintResources/ActorMacros.Switch Has Authority`
    (:`Authority`
      (`|AIMoveTo` null (0.0 0.0 0.0) (`self.Target`) (`BasicEnemy.AttackRadius` (cast `BasicEnemy` (`self.K2_GetPawn`) :!pure true))
        (:`OnSuccess`
          (`GameplayStatics.ApplyRadialDamage` :`BaseDamage` (`self.DamageAmount`) :`Origin` (`self.K2_GetActorLocation` (`self.K2_GetPawn`)) :`DamageRadius` 250.0 :`DamageTypeClass` "/Script/Engine.DamageType" :`DamageCauser` self :`InstigatedByController` (`self.GetInstigatorController`) :`bDoFullDamage` true))))
    (:`Remote`
      _))
  (`self.PlayExplosion`))

(event `PlayExplosion`
  (bind _asexplosive_enemy_bp (cast `/Game/Blueprints/Enemies/ExplosiveEnemy_BP` (`self.K2_GetPawn`)))
  (set `BasicEnemy.Health` -1.0 _asexplosive_enemy_bp))

(fn `UserConstructionScript`)