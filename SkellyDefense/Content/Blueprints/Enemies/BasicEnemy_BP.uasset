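; BasicEnemy_BP is a basic enemy character that attacks compass-direction walls and can be slowed.
; North, East and West attack events run on authority, calling the matching move on BasicEnemyAIController_BP; AttackSouth is empty, its logic disconnected.
; Tick displays Health on a text render and drops walk speed while Slowed, clearing it once SlowedTimer, which is never reset here, passes a threshold.
; The construction script creates a black body material instance.
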(event `self.AttackNorth`
  (`/Engine/EditorBlueprintResources/ActorMacros.Switch Has Authority`
    (:`Authority`
      (`KismetSystemLibrary.PrintString` "Attacking North")
      (bind _asbasic_enemy_aicontroller_bp (cast `/Game/Blueprints/Enemies/BasicEnemyAIController_BP` (`self.GetController`)))
      (`/Game/Blueprints/Enemies/BasicEnemyAIController_BP.MoveToNorthWall` _asbasic_enemy_aicontroller_bp))))

(event `self.AttackEast`
  (`/Engine/EditorBlueprintResources/ActorMacros.Switch Has Authority`
    (:`Authority`
      (`KismetSystemLibrary.PrintString` "Atttacking East")
      (bind _asbasic_enemy_aicontroller_bp (cast `/Game/Blueprints/Enemies/BasicEnemyAIController_BP` (`self.GetController`)))
      (`/Game/Blueprints/Enemies/BasicEnemyAIController_BP.MoveToEastWall` _asbasic_enemy_aicontroller_bp))))

(event `self.AttackSouth`)

(event `self.AttackWest`
  (`/Engine/EditorBlueprintResources/ActorMacros.Switch Has Authority`
    (:`Authority`
      (`KismetSystemLibrary.PrintString` "Attacking West")
      (bind _asbasic_enemy_aicontroller_bp (cast `/Game/Blueprints/Enemies/BasicEnemyAIController_BP` (`self.GetController`)))
      (`/Game/Blueprints/Enemies/BasicEnemyAIController_BP.MoveToWestWall` _asbasic_enemy_aicontroller_bp))))

(event `self.ReceiveBeginPlay`)

(event `self.ReceiveTick`
  (params (DeltaSeconds :type "Float (single-precision)"))
  (bind _charactermovement (`self.CharacterMovement`))
  (set `self.SlowedTimer` (+ (`self.SlowedTimer`) DeltaSeconds))
  (`TextRenderComponent.K2_SetText` (`self.TextRender`) (`KismetTextLibrary.Conv_StringToText` (`KismetStringLibrary.BuildString_Double` "" "Hello: " (`self.Health`))))
  (if (`self.Slowed`)
    (set `CharacterMovementComponent.MaxWalkSpeed` 50.0 _charactermovement)
    (if (>= (`self.SlowedTimer`) 10.0)
      (set `self.Slowed` false))
    (else
      (set `CharacterMovementComponent.MaxWalkSpeed` 300.0 _charactermovement))))

(fn `UserConstructionScript`
  (bind _returnvalue (`KismetMaterialLibrary.CreateDynamicMaterialInstance` "/Game/Mannequin/Character/Materials/M_UE4Man_Body.M_UE4Man_Body"))
  (`MaterialInstanceDynamic.SetVectorParameterValue` :`self` _returnvalue :`ParameterName` "BodyColor"))