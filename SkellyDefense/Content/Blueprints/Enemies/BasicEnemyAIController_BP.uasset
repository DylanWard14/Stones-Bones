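; AI controller for Skelly Defense basic enemies, sending them to attack their assigned wall, or the main building once that wall's health is depleted.
; Authority-only North, East and West events re-arm one-second timers to move and apply damage; South's logic is disconnected.
; Each tick of those timers first checks for players via sphere overlap and line trace, diverting to damage and chase any player found.
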(event `MoveToNorthWall`
  (bind _asbasic_enemy (cast `BasicEnemy` (`self.K2_GetPawn`) :!pure true))
  (bind _attackradius (`BasicEnemy.AttackRadius` _asbasic_enemy))
  (bind _item (`KismetArrayLibrary.Array_Get` (`SkellyDefenseGameMode.NorthWalls` (cast `/Game/Blueprints/SkellyDefenseGameMode_BP` (`GameplayStatics.GetGameMode`) :!pure true)) (`BasicEnemy.WallIndex` _asbasic_enemy)))
  (`/Engine/EditorBlueprintResources/ActorMacros.Switch Has Authority`
    (:`Authority`
      (`KismetSystemLibrary.K2_SetTimerDelegate` (delegate `MoveToNorthWall`) 1.0)
      (bind _canattackplayer (`self.CheckIfCanAttackPlayer` false))
      (if _canattackplayer
        (`self.AttackPlayer`)
        (elif (<= (`Wall.Health` _item) 0)
          (`|AIMoveTo` null (`self.K2_GetActorLocation` (`self.MainBuilding`)) null _attackradius
            (:`OnSuccess`
              (`GameplayStatics.ApplyDamage` (`self.MainBuilding`) (`self.DamageAmount`) (`self.GetInstigatorController`) self "/Script/Engine.DamageType")))
          (else
            (`|AIMoveTo` (`self.K2_GetPawn`) (`self.K2_GetActorLocation` _item) null _attackradius
              (:`OnSuccess`
                (`GameplayStatics.ApplyDamage` _item (`self.DamageAmount`) (`self.GetInstigatorController`) self "/Script/Engine.DamageType")))))))))

(event `MoveToSouthWall`)

(event `MoveToEastWall`
  (bind _asbasic_enemy (cast `BasicEnemy` (`self.K2_GetPawn`) :!pure true))
  (bind _attackradius (`BasicEnemy.AttackRadius` _asbasic_enemy))
  (bind _item (`KismetArrayLibrary.Array_Get` (`SkellyDefenseGameMode.EastWalls` (cast `/Game/Blueprints/SkellyDefenseGameMode_BP` (`GameplayStatics.GetGameMode`) :!pure true)) (`BasicEnemy.WallIndex` _asbasic_enemy)))
  (`/Engine/EditorBlueprintResources/ActorMacros.Switch Has Authority`
    (:`Authority`
      (`KismetSystemLibrary.K2_SetTimerDelegate` (delegate `MoveToEastWall`) 1.0)
      (bind _canattackplayer (`self.CheckIfCanAttackPlayer` false))
      (if _canattackplayer
        (`self.AttackPlayer`)
        (elif (<= (`Wall.Health` _item) 0)
          (`|AIMoveTo` null (`self.K2_GetActorLocation` (`self.MainBuilding`)) null _attackradius
            (:`OnSuccess`
              (`GameplayStatics.ApplyDamage` (`self.MainBuilding`) (`self.DamageAmount`) (`self.GetInstigatorController`) self "/Script/Engine.DamageType")))
          (else
            (`|AIMoveTo` (`self.K2_GetPawn`) (`self.K2_GetActorLocation` _item) null _attackradius
              (:`OnSuccess`
                (`GameplayStatics.ApplyDamage` _item (`self.DamageAmount`) (`self.GetInstigatorController`) self "/Script/Engine.DamageType")))))))))

(event `MoveToWestWall`
  (bind _asbasic_enemy (cast `BasicEnemy` (`self.K2_GetPawn`) :!pure true))
  (bind _attackradius (`BasicEnemy.AttackRadius` _asbasic_enemy))
  (bind _item (`KismetArrayLibrary.Array_Get` (`SkellyDefenseGameMode.WestWalls` (cast `/Game/Blueprints/SkellyDefenseGameMode_BP` (`GameplayStatics.GetGameMode`) :!pure true)) (`BasicEnemy.WallIndex` _asbasic_enemy)))
  (`/Engine/EditorBlueprintResources/ActorMacros.Switch Has Authority`
    (:`Authority`
      (`KismetSystemLibrary.K2_SetTimerDelegate` (delegate `MoveToWestWall`) 1.0)
      (bind _canattackplayer (`self.CheckIfCanAttackPlayer` false))
      (if _canattackplayer
        (`self.AttackPlayer`)
        (elif (<= (`Wall.Health` _item) 0)
          (`|AIMoveTo` null (`self.K2_GetActorLocation` (`self.MainBuilding`)) null _attackradius
            (:`OnSuccess`
              (`GameplayStatics.ApplyDamage` (`self.MainBuilding`) (`self.DamageAmount`) (`self.GetInstigatorController`) self "/Script/Engine.DamageType")))
          (else
            (`|AIMoveTo` (`self.K2_GetPawn`) (`self.K2_GetActorLocation` _item) null _attackradius
              (:`OnSuccess`
                (`GameplayStatics.ApplyDamage` _item (`self.DamageAmount`) (`self.GetInstigatorController`) self "/Script/Engine.DamageType")))))))))

(event `self.ReceiveBeginPlay`
  (bind _outactors (`GameplayStatics.GetAllActorsOfClass` "/Script/SkellyDefense.MainBuilding"))
  (set `self.MainBuilding` (`KismetArrayLibrary.Array_Get` _outactors))
  (`KismetSystemLibrary.Delay` 1.0)
  (set `self.DamageAmount` (`BasicEnemy.AttackDamage` (cast `BasicEnemy` (`self.K2_GetPawn`) :!pure true))))

(event `self.ReceiveTick`
  (params (DeltaSeconds :type "Float (single-precision)")))

(event `AttackPlayer`
  (bind (_canattackplayer _player) (`self.CheckIfCanAttackPlayer` true))
  (if _canattackplayer
    (`|AIMoveTo` (`self.K2_GetPawn`) (0.0 0.0 0.0) _player 50.0)))

(fn `CheckIfCanAttackPlayer`
  (params (ApplyDamage :type Boolean))
  (returns (CanAttackPlayer :type Boolean) (Player :type "Actor Object Reference"))
  (bind _outactors (`KismetSystemLibrary.SphereOverlapActors_NEW` (+ (`self.K2_GetActorLocation` (`self.K2_GetPawn`)) (`KismetMathLibrary.MakeVector` 85.0)) 160.0 (`|MakeArray` "ObjectTypeQuery3" :!type "EObjectTypeQuery Enum") "/Script/SkellyDefense.SkellyDefenseCharacter"))
  (if (>= (`KismetArrayLibrary.Array_Length` _outactors) 1)
    (bind _item (`KismetArrayLibrary.Array_Get` _outactors))
    (`/Engine/EditorBlueprintResources/StandardMacros.IsValid` _item
      (:`Is Valid`
        (bind _outhit (`KismetSystemLibrary.LineTraceSingle` :`Start` (`self.K2_GetActorLocation` (`self.K2_GetPawn`)) :`End` (`self.K2_GetActorLocation` _item) :`TraceChannel` "TraceTypeQuery1" :`DrawDebugType` "ForDuration"))
        (if (`GameplayStatics.BreakHitResult` _outhit)
          _
          (else
            (if ApplyDamage
              (`GameplayStatics.ApplyDamage` _item 20.0 (`self.GetInstigatorController`) self "/Script/Engine.DamageType"))
            (return true _item))))
      (:`Is Not Valid`
        _)))
  (return false null))

(fn `UserConstructionScript`)