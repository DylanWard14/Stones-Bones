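; Player-owned turret actor that automatically damages nearby enemies and decrements its owner's spawned-turret count when destroyed.
; Server-side overlap events maintain a list of actors tagged Enemy.
; A looping one-second server timer picks the first listed enemy with an unblocked Visibility trace to the barrel and applies damage directly, without projectiles.
; Tick smoothly interpolates the barrel's pitch and yaw toward the current target.
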(event `self.ReceiveDestroyed`
  (bind _owningplayer (`self.OwningPlayer`))
  (`/Engine/EditorBlueprintResources/ActorMacros.Switch Has Authority`
    (:`Authority`
      (set `Engineer.TurretsSpawned` (- (`Engineer.TurretsSpawned` _owningplayer) 1) _owningplayer))))

(event `self.ReceiveActorBeginOverlap`
  (params (OtherActor :type "Actor Object Reference"))
  (`/Engine/EditorBlueprintResources/ActorMacros.Switch Has Authority`
    (:`Authority`
      (if (`self.ActorHasTag` OtherActor "Enemy")
        (`KismetArrayLibrary.Array_Add` (`self.EnemiesInRange`) OtherActor)))))

(event `self.ReceiveBeginPlay`
  (`/Engine/EditorBlueprintResources/ActorMacros.Switch Has Authority`
    (:`Authority`
      (`KismetSystemLibrary.K2_SetTimerDelegate` (delegate `DamageFirst`) 1.0 true))))

(event `self.ReceiveActorEndOverlap`
  (params (OtherActor :type "Actor Object Reference"))
  (`/Engine/EditorBlueprintResources/ActorMacros.Switch Has Authority`
    (:`Authority`
      (if (`self.ActorHasTag` OtherActor "Enemy")
        (`KismetArrayLibrary.Array_RemoveItem` (`self.EnemiesInRange`) OtherActor)))))

(event `DamageFirst`
  (bind _enemiesinrange (`self.EnemiesInRange`))
  (set `self.hasTarget` false)
  (if (`KismetArrayLibrary.Array_IsValidIndex` _enemiesinrange)
    (for _index (range (`KismetArrayLibrary.Array_Length` _enemiesinrange))
      (if (`KismetArrayLibrary.Array_IsValidIndex` _enemiesinrange _index)
        (bind _outhit (`KismetSystemLibrary.LineTraceSingle` (`self.K2_GetActorLocation` (`KismetArrayLibrary.Array_Get` (`self.EnemiesInRange`) _index)) (`SceneComponent.K2_GetComponentLocation` (`self.Barrel`)) "TraceTypeQuery1"))
        (if (not (`GameplayStatics.BreakHitResult` _outhit))
          (set `self.hasTarget` true)
          (set `self.target` (`KismetArrayLibrary.Array_Get` (`self.EnemiesInRange`) _index))
          (break))))
    (if (`self.hasTarget`)
      (`GameplayStatics.ApplyDamage` (`self.target`) 1.0 (`self.GetInstigatorController`) self "/Script/Engine.DamageType"))))

(event `self.ReceiveTick`
  (params (DeltaSeconds :type "Float (single-precision)"))
  (bind _barrel (`self.Barrel`))
  (`/Engine/EditorBlueprintResources/ActorMacros.Switch Has Authority`
    (:`Authority`
      _)
    (:`Remote`
      _))
  (if (`KismetArrayLibrary.Array_IsValidIndex` (`self.EnemiesInRange`))
    (`/Engine/EditorBlueprintResources/StandardMacros.IsValid` (`self.target`)
      (:`Is Valid`
        (`SceneComponent.K2_SetWorldRotation` _barrel (`KismetMathLibrary.RInterpTo` (`SceneComponent.K2_GetComponentRotation` _barrel) (`KismetMathLibrary.MakeRotator` 0.0 (.pitch (`KismetMathLibrary.FindLookAtRotation` (`SceneComponent.K2_GetComponentLocation` _barrel) (`self.K2_GetActorLocation` (`self.target`)))) (.yaw (`KismetMathLibrary.FindLookAtRotation` (`SceneComponent.K2_GetComponentLocation` _barrel) (`self.K2_GetActorLocation` (`self.target`))))) (`GameplayStatics.GetWorldDeltaSeconds`) 3.0) false false)))))

(fn `DamageActor`)

(fn `UserConstructionScript`)