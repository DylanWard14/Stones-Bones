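; AI controller for Skelly Defense enemies that attack an assigned base wall, then target the main building once it falls.
; Four server-only events, one per compass side, look up the wall via the pawn's WallIndex in the GameMode's arrays.
; Each re-arms a one-second timer, moves to its target and applies damage on arrival; the main-building move leaves its Pawn input unset.
; BeginPlay caches the first MainBuilding found.
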(event `MoveToNorthWall`
  (bind _item (`KismetArrayLibrary.Array_Get` (`SkellyDefenseGameMode.NorthWalls` (cast `/Game/Blueprints/SkellyDefenseGameMode_BP` (`GameplayStatics.GetGameMode`) :!pure true)) (`BasicEnemy.WallIndex` (cast `/Game/Blueprints/BasicEnemy_BP` (`self.K2_GetPawn`) :!pure true))))
  (`/Engine/EditorBlueprintResources/ActorMacros.Switch Has Authority`
    (:`Authority`
      (`KismetSystemLibrary.K2_SetTimerDelegate` (delegate `MoveToNorthWall`) 1.0)
      (if (<= (`Wall.Health` _item) 0)
        (`|AIMoveTo` null (`self.K2_GetActorLocation` (`self.MainBuilding`))
          (:`OnSuccess`
            (`GameplayStatics.ApplyDamage` (`self.MainBuilding`) 10.0 (`self.GetInstigatorController`) self "/Script/Engine.DamageType")))
        (else
          (`|AIMoveTo` (`self.K2_GetPawn`) (`self.K2_GetActorLocation` _item) null 250.0
            (:`OnSuccess`
              (`GameplayStatics.ApplyDamage` _item 10.0 (`self.GetInstigatorController`) self "/Script/Engine.DamageType"))))))))

(event `MoveToSouthWall`
  (bind _item (`KismetArrayLibrary.Array_Get` (`SkellyDefenseGameMode.SouthWalls` (cast `/Game/Blueprints/SkellyDefenseGameMode_BP` (`GameplayStatics.GetGameMode`) :!pure true)) (`BasicEnemy.WallIndex` (cast `/Game/Blueprints/BasicEnemy_BP` (`self.K2_GetPawn`) :!pure true))))
  (`/Engine/EditorBlueprintResources/ActorMacros.Switch Has Authority`
    (:`Authority`
      (`KismetSystemLibrary.K2_SetTimerDelegate` (delegate `MoveToSouthWall`) 1.0)
      (if (<= (`Wall.Health` _item) 0)
        (`|AIMoveTo` null (`self.K2_GetActorLocation` (`self.MainBuilding`))
          (:`OnSuccess`
            (`GameplayStatics.ApplyDamage` (`self.MainBuilding`) 10.0 (`self.GetInstigatorController`) self "/Script/Engine.DamageType")))
        (else
          (`|AIMoveTo` (`self.K2_GetPawn`) (`self.K2_GetActorLocation` _item) null 250.0
            (:`OnSuccess`
              (`GameplayStatics.ApplyDamage` _item 10.0 (`self.GetInstigatorController`) self "/Script/Engine.DamageType"))))))))

(event `MoveToEastWall`
  (bind _item (`KismetArrayLibrary.Array_Get` (`SkellyDefenseGameMode.EastWalls` (cast `/Game/Blueprints/SkellyDefenseGameMode_BP` (`GameplayStatics.GetGameMode`) :!pure true)) (`BasicEnemy.WallIndex` (cast `/Game/Blueprints/BasicEnemy_BP` (`self.K2_GetPawn`) :!pure true))))
  (`/Engine/EditorBlueprintResources/ActorMacros.Switch Has Authority`
    (:`Authority`
      (`KismetSystemLibrary.K2_SetTimerDelegate` (delegate `MoveToEastWall`) 1.0)
      (if (<= (`Wall.Health` _item) 0)
        (`|AIMoveTo` null (`self.K2_GetActorLocation` (`self.MainBuilding`))
          (:`OnSuccess`
            (`GameplayStatics.ApplyDamage` (`self.MainBuilding`) 10.0 (`self.GetInstigatorController`) self "/Script/Engine.DamageType")))
        (else
          (`|AIMoveTo` (`self.K2_GetPawn`) (`self.K2_GetActorLocation` _item) null 250.0
            (:`OnSuccess`
              (`GameplayStatics.ApplyDamage` _item 10.0 (`self.GetInstigatorController`) self "/Script/Engine.DamageType"))))))))

(event `MoveToWestWall`
  (bind _item (`KismetArrayLibrary.Array_Get` (`SkellyDefenseGameMode.WestWalls` (cast `/Game/Blueprints/SkellyDefenseGameMode_BP` (`GameplayStatics.GetGameMode`) :!pure true)) (`BasicEnemy.WallIndex` (cast `/Game/Blueprints/BasicEnemy_BP` (`self.K2_GetPawn`) :!pure true))))
  (`/Engine/EditorBlueprintResources/ActorMacros.Switch Has Authority`
    (:`Authority`
      (`KismetSystemLibrary.K2_SetTimerDelegate` (delegate `MoveToWestWall`) 1.0)
      (if (<= (`Wall.Health` _item) 0)
        (`|AIMoveTo` null (`self.K2_GetActorLocation` (`self.MainBuilding`))
          (:`OnSuccess`
            (`GameplayStatics.ApplyDamage` (`self.MainBuilding`) 10.0 (`self.GetInstigatorController`) self "/Script/Engine.DamageType")))
        (else
          (`|AIMoveTo` (`self.K2_GetPawn`) (`self.K2_GetActorLocation` _item) null 250.0
            (:`OnSuccess`
              (`GameplayStatics.ApplyDamage` _item 10.0 (`self.GetInstigatorController`) self "/Script/Engine.DamageType"))))))))

(event `self.ReceiveBeginPlay`
  (bind _outactors (`GameplayStatics.GetAllActorsOfClass` "/Script/SkellyDefense.MainBuilding"))
  (set `self.MainBuilding` (`KismetArrayLibrary.Array_Get` _outactors)))

(fn `UserConstructionScript`)