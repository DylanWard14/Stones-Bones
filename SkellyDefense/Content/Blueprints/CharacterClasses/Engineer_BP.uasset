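; Engineer character class Blueprint that manages the player's health HUD and cleans up the turrets tied to the character.
; BeginPlay creates a HealthHUD widget and adds it to the viewport, and an UpdateHUD event forwards refreshes to it.
; On destruction it removes the HUD, destroys every actor in SpawnedTurrets and resets the turret count; turret spawning is not handled in these graphs.
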(event `self.ReceiveDestroyed`
  (`Widget.RemoveFromParent` (`self.HUD`))
  (for _array_element (`self.SpawnedTurrets`)
    (`self.K2_DestroyActor` _array_element))
  (set `self.TurretsSpawned` 0))

(event `self.BP_UpdateHUD`
  (`/Game/UI/HealthHUD.UpdateHUD` (`self.HUD`)))

(event `self.ReceiveBeginPlay`
  (bind _returnvalue (`|CreateWidget` "/Game/UI/HealthHUD.HealthHUD_C"))
  (bind _output_get (set `self.HUD` _returnvalue))
  (`UserWidget.AddToViewport` _output_get 0))

(fn `UserConstructionScript`)